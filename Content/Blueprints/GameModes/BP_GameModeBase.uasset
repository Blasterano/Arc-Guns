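; Base game mode Blueprint that puts the match's UI widgets on screen in response to game events.
; GameStart shows a start widget configured with the start delay, and GameOver shows an end widget with the win or loss result.
; GameScore and PlayerHealth share one path that creates and adds a new stats widget with score and health on every call, rather than updating an existing one.
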(event `self.GameStart`
  (bind _returnvalue (`|CreateWidget` "/Game/Blueprints/Widgets/WBP_GameStart.WBP_GameStart_C"))
  (`/Game/Blueprints/Widgets/WBP_GameStart.SetStartDelay` _returnvalue (`self.StartDelay`))
  (`UserWidget.AddToViewport` _returnvalue 0))

(event `self.GameOver`
  (params (PlayerWon :type Boolean))
  (bind _returnvalue (`|CreateWidget` "/Game/Blueprints/Widgets/WBP_GameEnd.WBP_GameEnd_C"))
  (`/Game/Blueprints/Widgets/WBP_GameEnd.SetPlayerResult` _returnvalue PlayerWon)
  (`UserWidget.AddToViewport` _returnvalue 0))

(event `self.GameScore`
  (params (Score :type Integer))
  (bind _returnvalue (`|CreateWidget` "/Game/Blueprints/Widgets/WBP_GameStats.WBP_GameStats_C" :!label _label))
  (`/Game/Blueprints/Widgets/WBP_GameStats.Set Stats` _returnvalue Score (stale `self.PlayerHealth` Health))
  (`UserWidget.AddToViewport` _returnvalue 0))

(event `self.PlayerHealth`
  (params (Health :type Integer))
  (goto _label))

(fn `UserConstructionScript`)